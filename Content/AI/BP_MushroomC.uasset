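; Mushroom AI character Blueprint that keeps track of its distance from the player.
; Every Tick it applies WalkSpeed to its movement component, then searches for the player-tagged ThirdPersonCharacter and stores the distance to the first match in DistFromPlayer, without a validity check.
; An unconnected branch, which never runs, would copy the player's walk speed when a Blackboard object value is valid.
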(event `self.ReceiveTick`
  (params (DeltaSeconds :type "Float (single-precision)"))
  (set `CharacterMovementComponent.MaxWalkSpeed` (`self.WalkSpeed`) (`self.CharacterMovement`))
  (bind _outactors (`GameplayStatics.GetAllActorsOfClassWithTag` "/Game/ThirdPerson/Blueprints/BP_ThirdPersonCharacter.BP_ThirdPersonCharacter_C" "Player"))
  (set `self.DistFromPlayer` (`KismetMathLibrary.VSize` (- (`self.K2_GetActorLocation` (`|GetArrayItem` _outactors)) (`self.K2_GetActorLocation`)))))

(fn `UserConstructionScript`)